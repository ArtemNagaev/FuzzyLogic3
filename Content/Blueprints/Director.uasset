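; Director simulates a business each Tick, deriving a balance change from cost, workers, production, salary and a Demand value randomized at BeginPlay.
; Check3Function does fuzzy-style classification, picking Low, Medium or High by whichever curve scores highest.
; Salary and Production levels form a rule matrix that sets MoodChange, zeroed without workers.
; Mood is classified using the Production curves; neither computed change is applied here.
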(event `self.ReceiveBeginPlay`
  (set `self.Demand` (`KismetMathLibrary.RandomFloatInRange` 60.0 100.0)))

(event `self.ReceiveTick`
  (params (DeltaSeconds :type "Float (single-precision)"))
  (bind _linguisticdescription (`self.Check3Function` (`self.Mood`) "/Game/Blueprints/Curves/Production/ProductionLow.ProductionLow" "/Game/Blueprints/Curves/Production/ProductionMedium.ProductionMedium" "/Game/Blueprints/Curves/Production/ProductionHigh.ProductionHigh"))
  (set `self.MoodEnum` _linguisticdescription)
  (set `self.BalanceChange` (- (* (* (`self.Cost`) (* (`self.WorkersCount`) (`self.Production`))) (`self.Demand`)) (* (`self.WorkersCount`) (`self.Salary`))))
  (`|ExecutionSequence`
    (:`then_0`
      (bind _linguisticdescription_2 (`self.Check3Function` (`self.Salary`) "/Game/Blueprints/Curves/Salary/SalaryLow.SalaryLow" "/Game/Blueprints/Curves/Salary/SalaryMedium.SalaryMedium" "/Game/Blueprints/Curves/Salary/SalaryHigh.SalaryHigh"))
      (if (> (`self.WorkersCount`) 0)
        (switch `/Game/Blueprints/LowMediumHigh` _linguisticdescription_2
          (:`NewEnumerator0`
            (bind _linguisticdescription_3 (`self.Check3Function` (`self.Production`) "/Game/Blueprints/Curves/Production/ProductionLow.ProductionLow" "/Game/Blueprints/Curves/Production/ProductionMedium.ProductionMedium" "/Game/Blueprints/Curves/Production/ProductionHigh.ProductionHigh"))
            (switch `/Game/Blueprints/LowMediumHigh` _linguisticdescription_3
              (:`NewEnumerator0`
                (set `self.MoodChange` 0.0))
              (:`NewEnumerator1`
                (set `self.MoodChange` -50.0))
              (:`NewEnumerator2`
                (set `self.MoodChange` -50.0))))
          (:`NewEnumerator1`
            (bind _linguisticdescription_4 (`self.Check3Function` (`self.Production`) "/Game/Blueprints/Curves/Production/ProductionLow.ProductionLow" "/Game/Blueprints/Curves/Production/ProductionMedium.ProductionMedium" "/Game/Blueprints/Curves/Production/ProductionHigh.ProductionHigh"))
            (switch `/Game/Blueprints/LowMediumHigh` _linguisticdescription_4
              (:`NewEnumerator0`
                (set `self.MoodChange` 50.0))
              (:`NewEnumerator1`
                (set `self.MoodChange` 0.0))
              (:`NewEnumerator2`
                (set `self.MoodChange` -50.0))))
          (:`NewEnumerator2`
            (bind _linguisticdescription_5 (`self.Check3Function` (`self.Production`) "/Game/Blueprints/Curves/Production/ProductionLow.ProductionLow" "/Game/Blueprints/Curves/Production/ProductionMedium.ProductionMedium" "/Game/Blueprints/Curves/Production/ProductionHigh.ProductionHigh"))
            (switch `/Game/Blueprints/LowMediumHigh` _linguisticdescription_5
              (:`NewEnumerator0`
                (set `self.MoodChange` 50.0))
              (:`NewEnumerator1`
                (set `self.MoodChange` 50.0))
              (:`NewEnumerator2`
                (set `self.MoodChange` 0.0)))))
        (else
          (set `self.MoodChange` 0.0))))))

(fn `Check3Function`
  (params (Value :type "Float (double-precision)") (LowCurve :type "CurveFloat Object Reference") (MediumCurve :type "CurveFloat Object Reference") (HardCurve :type "CurveFloat Object Reference"))
  (returns (LinguisticDescription :type "/Game/Blueprints/LowMediumHigh Enum"))
  (locals (LowLocal :type "CurveFloat Object Reference") (ValueLocal :type "Float (double-precision)") (MediumLocal :type "CurveFloat Object Reference") (HighLocal :type "CurveFloat Object Reference") (MaxValueLocal :type "Float (double-precision)"))
  (set `local.ValueLocal` Value)
  (set `local.LowLocal` LowCurve)
  (set `local.MediumLocal` MediumCurve)
  (set `local.HighLocal` HardCurve)
  (set `local.MaxValueLocal` (`KismetMathLibrary.FMax` (`CurveFloat.GetFloatValue` (`local.LowLocal`) (`local.ValueLocal`)) (`CurveFloat.GetFloatValue` (`local.MediumLocal`) (`local.ValueLocal`)) (`CurveFloat.GetFloatValue` (`local.HighLocal`) (`local.ValueLocal`))))
  (if (== (`local.MaxValueLocal`) (`CurveFloat.GetFloatValue` (`local.LowLocal`) (`local.ValueLocal`)))
    (return "NewEnumerator0")
    (elif (== (`local.MaxValueLocal`) (`CurveFloat.GetFloatValue` (`local.MediumLocal`) (`local.ValueLocal`)))
      (return "NewEnumerator1")
      (elif (== (`local.MaxValueLocal`) (`CurveFloat.GetFloatValue` (`local.HighLocal`) (`local.ValueLocal`)))
        (return "NewEnumerator2")
        (else
          (return "NewEnumerator3"))))))

(fn `UserConstructionScript`)